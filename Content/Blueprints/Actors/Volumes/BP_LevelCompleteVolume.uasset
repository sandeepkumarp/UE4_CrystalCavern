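; Level-exit trigger volume that moves the player to the next level when overlapped, or quits the game on the final one.
; It gates completion on a count of BP_CrystalBase actors, but AnyCrystalsRemaining returns true when none exist, so as written completion runs only while crystals remain.
; Level order comes from the LevelNames array, indexed by the current level's name.
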(event Collision|EventActorBeginOverlap
  (params (OtherActor :type Actor%20Object%20Reference))
  (Utilities|IsPlayer OtherActor
    (:true
      (if (CallFunction|AnyCrystalsRemaining)
        (Development|PrintString "Crystals still remaining")
        (else
          (LevelManagerment|CompleteLevel))))))

(fn ConstructionScript)

(fn AnyCrystalsRemaining
  (bind _outactors (Actor|GetAllActorsOfClass "/Game/Blueprints/Actors/Collectables/BP_CrystalBase.BP_CrystalBase_C"))
  (return (== (Utilities|Array|Length _outactors) 0)))

(fn CompleteLevel
  (if (LevelManagerment|IsFinalLevel)
    (Game|QuitGame 0 "Quit" false)
    (else
      (LevelManagerment|LoadNextLevel))))

(fn GetCurrentLevelIndex
  (bind _returnvalue (Game|GetCurrentLevelName true))
  (return (Utilities|Array|FindItem (Variables|Default|GetLevelNames) (Utilities|String|StringToName _returnvalue))))

(fn IsFinalLevel
  (return (== (Utilities|Array|LastIndex (Variables|Default|GetLevelNames)) (LevelManagerment|GetCurrentLevelIndex))))

(fn LoadNextLevel
  (Game|OpenLevel(byName) (LevelManagerment|GetNextLevelName)))

(fn GetNextLevelName
  (return (Utilities|Array|Get(acopy) (Variables|Default|GetLevelNames) (+ (LevelManagerment|GetCurrentLevelIndex) 1))))