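; BP_Crystal is a collectable crystal that flies into the player pawn on overlap, then destroys itself.
; On BeginPlay it creates a dynamic instance of the blue crystal material and copies its Color parameter to the crystal's light.
; On player overlap it stores its location and plays a timeline whose alpha lerps it toward the pawn's current position, so it tracks a moving player.
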(event EventBeginPlay
  (bind _returnvalue (Rendering|Material|CreateDynamicMaterialInstance (Variables|Default|GetStaticMesh) 0 "/Game/Maetrials/MI_Crystal_Blue.MI_Crystal_Blue" "None" :!class /Script/Engine.PrimitiveComponent))
  (bind _returnvalue_2 (Rendering|Material|GetVectorParameterValue _returnvalue "Color" :!class /Script/Engine.MaterialInstanceDynamic))
  (Rendering|Components|Light|SetLightColor (Variables|Default|GetCrystalLight) _returnvalue_2 true))

(event Collision|EventActorBeginOverlap
  (params (OtherActor :type Actor%20Object%20Reference))
  (bind _returnvalue (Game|Player|GetPlayerPawn 0))
  (if (== OtherActor _returnvalue)
    (Variables|Default|SetLerpStartLocation (Transformation|GetActorLocation))
    (bind _smoothlerpalpha (Timeline|Timeline_AlphaBlend Play)
      (:Update
        (Transformation|SetActorLocation (Math|Vector|Lerp(Vector) (Variables|Default|GetLerpStartLocation) (Transformation|GetActorLocation _returnvalue) _smoothlerpalpha) false false))
      (:Finished
        (Actor|DestroyActor)))))

(fn ConstructionScript)